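; Fan trap for a 2D pixel platformer that periodically switches on and off and lifts the player while active.
; A looping timer drives a FlipFlop that toggles the active flag, flipbook animation and Niagara effect.
; Tick launches an overlapping player upward with reduced gravity and Flying movement mode.
; Ending the overlap restores gravity scale but does not explicitly reset the movement mode.
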(event OnComponentEndOverlap(CollisionDetectPlayer)
  (params (OverlappedComponent :type Primitive%20Component%20Object%20Reference) (OtherActor :type Actor%20Object%20Reference) (OtherComp :type Primitive%20Component%20Object%20Reference) (OtherBodyIndex :type Integer))
  (bind _as_bp_player (CallFunction|GetPlayerReference))
  (if (== OtherActor _as_bp_player)
    (Variables|/Script/Engine.CharacterMovementComponent|SetGravityScale (Variables|/Script/Engine.Character|GetCharacterMovement _as_bp_player) 1.0)))

(event Custom|toggleStatusFan
  (Utilities|FlowControl|FlipFlop
    (:A
      (Variables|Default|SetbActive true)
      (Components|Timeline|SetPlayRate (Variables|Default|GetPaperFlipbook) 1.0)
      (Development|SetHiddeninGame (Variables|Default|GetNiagara) false false))
    (:B
      (Variables|Default|SetbActive false)
      (Components|Timeline|SetPlayRate (Variables|Default|GetPaperFlipbook) 0.0)
      (Development|SetHiddeninGame (Variables|Default|GetNiagara) true false))))

(event EventTick
  (params (DeltaSeconds :type Float%20%28single-precision%29))
  (bind _as_bp_player (CallFunction|GetPlayerReference))
  (bind _charactermovement (Variables|/Script/Engine.Character|GetCharacterMovement _as_bp_player))
  (if (and (Collision|IsOverlappingActor (Variables|Default|GetCollisionDetectPlayer) _as_bp_player :!class /Script/Engine.PrimitiveComponent) (Variables|Default|GetbActive))
    (Variables|/Script/Engine.CharacterMovementComponent|SetGravityScale _charactermovement 0.5)
    (Character|LaunchCharacter _as_bp_player (Math|Vector|MakeVector 0.0 0.0 75.0) false true)
    (Pawn|Components|CharacterMovement|SetMovementMode _charactermovement "MOVE_Flying" 0)))

(event EventBeginPlay
  (Utilities|Time|SetTimerbyEvent (delegate Custom|toggleStatusFan) (Variables|Default|GetsecondsToggleStatus) true))

(fn ConstructionScript)