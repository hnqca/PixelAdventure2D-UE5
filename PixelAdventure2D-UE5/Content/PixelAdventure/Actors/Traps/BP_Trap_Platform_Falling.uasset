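; Falling platform trap that hovers vertically until the player overlaps it, then drops away.
; A timeline started on BeginPlay lerps the actor's Z from its spawn height toward a configurable offset.
; Player overlap stops that timeline, freezes the flipbook animation and starts a configurable timer.
; When the timer fires, the box switches to physics-only simulation, receives an impulse and the actor is destroyed shortly after.
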(event Custom|startFlyMovement
  (bind _originalactorlocation (Variables|Default|GetoriginalActorLocation))
  (bind _transition (Timeline|Timeline_FlyMovement PlayFromStart)
    (:Update
      (Transformation|SetActorLocation (Math|Vector|MakeVector (.x _originalactorlocation) (.y _originalactorlocation) (Math|Float|Lerp (.z _originalactorlocation) (+ (.z (Variables|Default|GetoriginalActorLocation)) (Variables|Default|GetNew%20Location%20Z)) _transition)) false false))))

(event Custom|onDesactivePlatform
  (bind _box (Variables|Default|GetBox))
  (Utilities|FlowControl|Sequence
    (:then_0
      (Physics|SetSimulatePhysics _box true)
      (Collision|SetCollisionEnabled _box "PhysicsOnly")
      (Physics|AddImpulse _box "0.000000,110.000000,0.000000" "None" true)
      (Utilities|FlowControl|Delay 3.0)
      (Actor|DestroyActor))))

(event EventBeginPlay
  (Variables|Default|SetoriginalActorLocation (Transformation|GetActorLocation))
  (CallFunction|StartFlyMovement))

(event Collision|EventActorBeginOverlap
  (params (OtherActor :type Actor%20Object%20Reference))
  (if (== OtherActor (CallFunction|GetPlayerReference))
    (Audio|Components|Audio|Stop (Variables|Default|GetTimeline_FlyMovement))
    (Components|Timeline|SetPlayRate (Variables|Default|GetPaperFlipbook) 0.0)
    (Utilities|Time|SetTimerbyEvent (delegate Custom|onDesactivePlatform) (Variables|Default|GettimeToDesactivePlatform%20%28in%20seconds%29))))

(fn ConstructionScript)