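; Fire trap for the Pixel Adventure game that turns on when something overlaps its detection area and damages overlapping actors while lit.
; Activation plays the hit flipbook, switches to the fire loop, sets IsActive, checks existing overlaps and starts a timer to switch off.
; New overlaps and the existing-overlap loop share one damage branch, which targets the overlap event's OtherActor rather than the loop element.
; Collision-toggling nodes are disconnected.
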(event OnComponentBeginOverlap(CollisionDetectPawn)
  (params (OverlappedComponent :type Primitive%20Component%20Object%20Reference) (OtherActor :type Actor%20Object%20Reference) (OtherComp :type Primitive%20Component%20Object%20Reference) (OtherBodyIndex :type Integer) (bFromSweep :type Boolean) (SweepResult :type Hit%20Result%20Structure%20%28by%20ref%29))
  ;[0 0 0 1 22] Ativa a armadilha ao detectar algum "pawn" na área de colissão
  (if (not (Variables|Default|GetbIsActive))
    (CallFunction|Active)))

(event OnComponentBeginOverlap(CollisionApplyDamage)
  (params (OverlappedComponent :type Primitive%20Component%20Object%20Reference) (OtherActor :type Actor%20Object%20Reference) (OtherComp :type Primitive%20Component%20Object%20Reference) (OtherBodyIndex :type Integer) (bFromSweep :type Boolean) (SweepResult :type Hit%20Result%20Structure%20%28by%20ref%29))
  ;[0 0 0 1 22] Aplica dano ao "pawn" detectado
  (if (Variables|Default|GetbIsActive)
    (Game|Damage|ApplyDamage OtherActor 1.0 0 0)))

(event Custom|active
  (bind _paperflipbook (Variables|Default|GetPaperFlipbook))
  ;[0 0.6627 0.01961 1 22] Ativação da armadilha
  (Sprite|SetFlipbook _paperflipbook "/Game/PixelAdventure/Assets/Traps/Fire/hit/FB_Trap_Fire_Hit.FB_Trap_Fire_Hit")
  (Utilities|FlowControl|Delay (Class|PaperFlipbookComponent|GetFlipbookLength _paperflipbook))
  (Sprite|SetFlipbook _paperflipbook "/Game/PixelAdventure/Assets/Traps/Fire/on/FB_Trap_Fire_On.FB_Trap_Fire_On")
  (Variables|Default|SetbIsActive true)
  (CallFunction|CheckPawnOverlapping)
  ;[0.6627 0.3588 0] Aguarda X segundos para desativar a armadilha
  (Utilities|Time|SetTimerbyEvent (delegate Custom|desactive) (Variables|Default|GetTimeToDesactive%20%28in%20seconds%29)))

(event Custom|desactive
  ;[0.6627 0.01645 0 1 22] Desativação da Armadilha
  (Sprite|SetFlipbook (Variables|Default|GetPaperFlipbook) "/Game/PixelAdventure/Assets/Traps/Fire/off/FB_Trap_Fire_Off.FB_Trap_Fire_Off")
  (Variables|Default|SetbIsActive false))

(event Custom|checkPawnOverlapping
  ;[0 0 0 1 22] Aplica dano ao "pawn" detectado
  (for _array_element (Collision|GetOverlappingActors (Variables|Default|GetCollisionApplyDamage) "/Script/PaperZD.PaperZDCharacter" :!class /Script/Engine.PrimitiveComponent)
    (Utilities|IsValid _array_element
      (:Is%20Valid
        (if (Variables|Default|GetbIsActive)
          (Game|Damage|ApplyDamage (stale OnComponentBeginOverlap(CollisionApplyDamage) OtherActor) 1.0 0 0))))))

(fn ConstructionScript)