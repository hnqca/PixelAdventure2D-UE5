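; Breakable brick block that bounces when the player overlaps its head-detection collider and breaks after a set number of hits.
; A DoOnce with a short reset delay debounces overlaps, counts each hit and replays a timeline that moves the sprite on Z.
; Once the hit limit is reached, the bounce update plays a destroy sound, spawns a Niagara break effect and destroys the actor.
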(event OnComponentBeginOverlap(CollisionDetectHeadPlayer)
  (params (OverlappedComponent :type Primitive%20Component%20Object%20Reference) (OtherActor :type Actor%20Object%20Reference) (OtherComp :type Primitive%20Component%20Object%20Reference) (OtherBodyIndex :type Integer) (bFromSweep :type Boolean) (SweepResult :type Hit%20Result%20Structure%20%28by%20ref%29))
  (bind _returnvalue (Transformation|GetActorLocation))
  (if (== OtherActor (CallFunction|GetPlayerReference))
    (Utilities|FlowControl|DoOnce false :!label _label
      (:Completed
        (Utilities|FlowControl|Sequence
          (:then_0
            (Utilities|FlowControl|Delay 0.2)
            (goto _label Reset))
          (:then_1
            (Math|Integer|IncrementInt (Variables|Default|GetamountHits)
              (:%20%20
                (bind _locationz (Timeline|Timeline PlayFromStart)
                  (:Update
                    (Transformation|SetRelativeLocation (Variables|Default|GetPaperSprite) (Math|Vector|MakeVector 0.0 0.0 _locationz) false false)
                    (if (and (>= _locationz 0.3) (>= (Variables|Default|GetamountHits) (Variables|Default|GetquantityHitsToDestroy)))
                      (Utilities|FlowControl|DoOnce false
                        (:Completed
                          (Audio|PlaySound2D "/Game/PixelAdventure/Assets/Audio/Effects/destroy.destroy" 1.0 1.0 0.0 0 0)
                          (Niagara|SpawnSystematLocation "/Game/PixelAdventure/Assets/Effects/Niagara/NS_BreakBlock.NS_BreakBlock" (Math|Vector|MakeVector (.x _returnvalue) -1e+01 (.z _returnvalue)) "0, 0, 0" "0.300000,0.300000,0.300000")
                          (Actor|DestroyActor))))))))))))))

(event EventBeginPlay)

(event Collision|EventActorBeginOverlap
  (params (OtherActor :type Actor%20Object%20Reference)))

(event EventTick
  (params (DeltaSeconds :type Float%20%28single-precision%29)))

(fn ConstructionScript)