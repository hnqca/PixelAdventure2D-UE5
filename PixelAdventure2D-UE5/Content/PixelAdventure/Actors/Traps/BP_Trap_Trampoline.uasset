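; BP_Trap_Trampoline is a trampoline trap for the Pixel Adventure game that bounces the player on contact.
; When the player overlaps the detection collision, it launches the character with LaunchVelocity, overriding only Z velocity, and plays a 2D sound.
; It then switches its Paper2D flipbook to the jump animation and uses a delay of that flipbook's length to return to idle.
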(event OnComponentBeginOverlap(collisionDetectPlayer)
  (params (OverlappedComponent :type Primitive%20Component%20Object%20Reference) (OtherActor :type Actor%20Object%20Reference) (OtherComp :type Primitive%20Component%20Object%20Reference) (OtherBodyIndex :type Integer) (bFromSweep :type Boolean) (SweepResult :type Hit%20Result%20Structure%20%28by%20ref%29))
  (bind _as_bp_player (CallFunction|GetPlayerReference))
  (bind _paperflipbook (Variables|Default|GetPaperFlipbook))
  (if (== OtherActor _as_bp_player)
    (Utilities|FlowControl|Sequence
      (:then_0
        (Character|LaunchCharacter _as_bp_player (Variables|Default|GetLaunchVelocity) false true)
        (Audio|PlaySound2D "/Game/PixelAdventure/Assets/Audio/Effects/trampoline.trampoline" 1.0 1.0 0.0 0 0))
      (:then_1
        (Sprite|SetFlipbook _paperflipbook "/Game/PixelAdventure/Assets/Traps/Trampoline/jump/FB_Trap_Trampoline_Jump.FB_Trap_Trampoline_Jump")
        (Utilities|FlowControl|Delay (Class|PaperFlipbookComponent|GetFlipbookLength _paperflipbook))
        (Sprite|SetFlipbook _paperflipbook "/Game/PixelAdventure/Assets/Traps/Trampoline/idle/FB_Trap_Trampoline_Idle.FB_Trap_Trampoline_Idle")))))

(fn ConstructionScript)