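; Moving platform trap for a Paper2D platformer, carrying its flipbook along a spline from BeginPlay.
; A timeline, rate-scaled to the configured duration, maps its value to spline distance.
; A FlipFlop alternates play and reverse, re-triggered on finish when looping, so the platform ping-pongs.
; With the chain option on, the construction script lays non-colliding chain sprites at fixed intervals along the spline.
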(event Custom|startSplineMovement
  (bind _spline (Variables|Default|GetSpline))
  (Components|Timeline|SetPlayRate (Variables|Default|GetTimeline_SplineMovement) (/ 1.0 (Variables|Default|GetdurationSplineMovement%20%28in%20seconds%29)))
  (Utilities|FlowControl|FlipFlop
    (:A
      (bind _transition (Timeline|Timeline_SplineMovement Play)
        (:Update
          (Transformation|SetWorldLocation (Variables|Default|GetPaperFlipbook) (Spline|GetLocationatDistanceAlongSpline _spline (* _transition (Spline|GetSplineLength _spline)) "World") false false))
        (:Finished
          (if (Variables|Default|GetisLoopMovement)
            (CallFunction|StartSplineMovement)))))
    (:B
      (Timeline|Timeline_SplineMovement Reverse))))

(event EventBeginPlay
  (CallFunction|StartSplineMovement))

(event Collision|EventActorBeginOverlap
  (params (OtherActor :type Actor%20Object%20Reference)))

(event EventTick
  (params (DeltaSeconds :type Float%20%28single-precision%29)))

(fn ConstructionScript
  (if (Variables|Default|GetwithChain)
    (CallFunction|SetChainTrail)))

(fn SetChainTrail
  (for _index (range 0 (Math|Float|Floor (/ (Spline|GetSplineLength (Variables|Default|GetSpline)) (Variables|Default|GetoffsetChain))))
    (bind _returnvalue (AddComponent|AddPaperSpriteComponent false (Math|Conversions|ToTransform(Vector) (- (Spline|GetLocationatDistanceAlongSpline (Variables|Default|GetSpline) (* _index (Variables|Default|GetoffsetChain)) "Local") "0.000000,2.000000,0.000000"))))
    (Rendering|Components|Sprite|SetSprite _returnvalue (Variables|Default|GetchainSprite))
    (Collision|SetCollisionEnabled _returnvalue "NoCollision")))