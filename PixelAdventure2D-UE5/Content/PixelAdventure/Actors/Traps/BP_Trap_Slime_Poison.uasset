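; Poison trap actor of the slime trap set that damages the player on contact and removes itself after its animation.
; Shortly after BeginPlay, it sets the flipbook to non-looping, waits one flipbook length, then runs a timeline that drives all sprite color channels, alpha included, and destroys the actor when finished.
; Overlap on the damage collision applies damage only to the player, limited to a single hit by a DoOnce.
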(event OnComponentBeginOverlap(CollisionApplyDamage)
  (params (OverlappedComponent :type Primitive%20Component%20Object%20Reference) (OtherActor :type Actor%20Object%20Reference) (OtherComp :type Primitive%20Component%20Object%20Reference) (OtherBodyIndex :type Integer) (bFromSweep :type Boolean) (SweepResult :type Hit%20Result%20Structure%20%28by%20ref%29))
  (bind _as_bp_player (CallFunction|GetPlayerReference))
  (if (== OtherActor _as_bp_player)
    (Utilities|FlowControl|DoOnce false
      (:Completed
        (Game|Damage|ApplyDamage _as_bp_player 1.0 0 0)))))

(event EventBeginPlay
  (bind _paperflipbook (Variables|Default|GetPaperFlipbook))
  (Utilities|FlowControl|Delay 0.2)
  (Components|Timeline|SetLooping _paperflipbook false)
  (Components|Timeline|SetPlayRate _paperflipbook 1.0)
  (Utilities|FlowControl|Delay (Class|PaperFlipbookComponent|GetFlipbookLength _paperflipbook))
  (bind _newtrack_0 (Timeline|Timeline PlayFromStart)
    (:Update
      (Sprite|SetSpriteColor (Variables|Default|GetPaperFlipbook) (Utilities|Struct|MakeLinearColor _newtrack_0 _newtrack_0 _newtrack_0 _newtrack_0)))
    (:Finished
      (Actor|DestroyActor))))

(event Collision|EventActorBeginOverlap
  (params (OtherActor :type Actor%20Object%20Reference)))

(event EventTick
  (params (DeltaSeconds :type Float%20%28single-precision%29)))

(fn ConstructionScript)