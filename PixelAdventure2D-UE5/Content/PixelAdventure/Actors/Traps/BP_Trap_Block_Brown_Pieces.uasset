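; Debris actor for the brown block trap in the pixel adventure game, showing two broken pieces flying apart before removing itself.
; On BeginPlay, two paper sprites get randomized velocity-change impulses, upward and in opposite horizontal directions.
; After a short delay, a timeline drives all RGBA channels of both sprites' color from one track, then destroys the actor when finished.
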(event EventBeginPlay
  (Utilities|FlowControl|Sequence
    (:then_0
      (Physics|AddImpulse (Variables|Default|GetPaperSprite_2) (Math|Vector|MakeVector (Math|Random|RandomFloatinRange -5e+01 -1e+02) 0.0 (Math|Random|RandomFloatinRange 1.2e+02 2.5e+02)) "None" true))
    (:then_1
      (Physics|AddImpulse (Variables|Default|GetPaperSprite_1) (Math|Vector|MakeVector (Math|Random|RandomFloatinRange 5e+01 1e+02) 0.0 (Math|Random|RandomFloatinRange 9e+01 2e+02)) "None" true))
    (:then_2
      (Utilities|FlowControl|Delay 1.5)
      (bind _newtrack_0 (Timeline|Timeline Play)
        (:Update
          (Sprite|SetSpriteColor (Variables|Default|GetPaperSprite_2) (Utilities|Struct|MakeLinearColor _newtrack_0 _newtrack_0 _newtrack_0 _newtrack_0))
          (Sprite|SetSpriteColor (Variables|Default|GetPaperSprite_1) (Utilities|Struct|MakeLinearColor _newtrack_0 _newtrack_0 _newtrack_0 _newtrack_0)))
        (:Finished
          (Actor|DestroyActor))))))

(fn ConstructionScript)