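; Breakable brown block trap that reacts once when its player-detection collision is overlapped, then shatters.
; On overlap it immediately launches the referenced player, calls the player's camera shake and damage function, and plays a damage sound.
; In parallel it plays the top-hit flipbook, waits for that flipbook's length, spawns the block pieces actor at the sprite's transform and destroys itself.
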(event OnComponentBeginOverlap(CollisionDetectPlayer)
  (params (OverlappedComponent :type Primitive%20Component%20Object%20Reference) (OtherActor :type Actor%20Object%20Reference) (OtherComp :type Primitive%20Component%20Object%20Reference) (OtherBodyIndex :type Integer) (bFromSweep :type Boolean) (SweepResult :type Hit%20Result%20Structure%20%28by%20ref%29))
  (bind _as_bp_player (CallFunction|GetPlayerReference))
  (bind _paperflipbook (Variables|Default|GetPaperFlipbook))
  (Utilities|FlowControl|DoOnce false
    (:Completed
      (Utilities|FlowControl|Sequence
        (:then_0
          (Sprite|SetFlipbook _paperflipbook "/Game/PixelAdventure/Assets/Traps/Blocks/Brown/HitTop/FB_Trap_Blocks_Brown_HitTop.FB_Trap_Blocks_Brown_HitTop")
          (Utilities|FlowControl|Delay (Class|PaperFlipbookComponent|GetFlipbookLength _paperflipbook))
          (Game|SpawnActorfromClass "/Game/PixelAdventure/Actors/Traps/BP_Trap_Block_Brown_Pieces.BP_Trap_Block_Brown_Pieces_C" (Transformation|GetWorldTransform (Variables|Default|GetPaperFlipbook)) "Undefined" "MultiplyWithRoot" 0 0)
          (Actor|DestroyActor))
        (:then_1
          (Default|Launch _as_bp_player 1.05)
          (Default|StartCameraShakeApplyDamage _as_bp_player)
          (Audio|PlaySound2D "/Game/PixelAdventure/Assets/Audio/Effects/enemyDamage.enemyDamage" 1.0 1.0 0.0 0 0))))))

(event EventBeginPlay)

(event Collision|EventActorBeginOverlap
  (params (OtherActor :type Actor%20Object%20Reference)))

(event EventTick
  (params (DeltaSeconds :type Float%20%28single-precision%29)))

(fn ConstructionScript)