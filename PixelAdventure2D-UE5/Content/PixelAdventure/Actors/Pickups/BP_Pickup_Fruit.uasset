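; BP_Pickup_Fruit is a collectible fruit pickup that picks a random fruit flipbook on BeginPlay.
; On first player overlap, it adds one fruit to the player, plays a sound and swaps to a collected effect.
; After the effect's length it destroys itself, then counts remaining fruit actors in the level.
; When none remain, it enables the flag on the BP_Checkpoint, so the last pickup completes the collection goal.
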(event OnComponentBeginOverlap(CollisionPlayerDetection)
  (params (OverlappedComponent :type Primitive%20Component%20Object%20Reference) (OtherActor :type Actor%20Object%20Reference) (OtherComp :type Primitive%20Component%20Object%20Reference) (OtherBodyIndex :type Integer) (bFromSweep :type Boolean) (SweepResult :type Hit%20Result%20Structure%20%28by%20ref%29))
  (bind _as_bp_player (CallFunction|GetPlayerReference))
  (bind _paperflipbook (Variables|Default|GetPaperFlipbook))
  ;[1 1 1 1 30] Player Collect Fruit
  (if (== OtherActor _as_bp_player)
    (Utilities|FlowControl|DoOnce false
      (:Completed
        (Utilities|FlowControl|Sequence
          (:then_0
            ;;[1 1 1] Effect upon collecting the fruit and actor destruction
            (Sprite|SetFlipbook _paperflipbook "/Game/PixelAdventure/Assets/Effects/Flipbooks/CollectedPickup/FB_Effect_Collected.FB_Effect_Collected")
            (Utilities|FlowControl|Delay (Class|PaperFlipbookComponent|GetFlipbookLength _paperflipbook))
            (Actor|DestroyActor)
            ;;[1 1 1] check if all the fruits in the level have been collected.
            (if (== (CallFunction|GetTotalFruitstoFinishLevel) 0)
              ;;[1 1 1] if true, activate the flag.
              (bind _returnvalue (Actor|GetActorOfClass "/Game/PixelAdventure/Actors/Interactables/BP_Checkpoint.BP_Checkpoint_C"))
              (Default|EnableFlag _returnvalue)))
          (:then_1
            (Default|AddFruit _as_bp_player 1)
            (Audio|PlaySound2D "/Game/PixelAdventure/Assets/Audio/Effects/collected.collected" 1.0 1.0 0.0 0 0)))))))

(event EventBeginPlay
  (CallFunction|SetRandomFlipbookFruit))

(fn ConstructionScript
  (|CallParentFunction))

(fn GetTotalFruitstoFinishLevel
  (bind _outactors (Actor|GetAllActorsOfClass "BP_Pickup_Fruit_C"))
  (return (Utilities|Array|Length _outactors)))

(fn SetRandomFlipbookFruit
  (Sprite|SetFlipbook (Variables|Default|GetPaperFlipbook) (.OutItem (Utilities|Array|Random (Variables|Default|Getfruits)))))