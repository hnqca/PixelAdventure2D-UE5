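; BP_Checkpoint is the level-end flag that finishes the current level when the player reaches it.
; enableFlag activates it, playing the raise flipbook before switching to idle.
; The first player overlap while active updates the loaded save game's level and fruits, disables player damage and plays the victory sound.
; A timeline drives a material parameter collection transition, then opens the next level by its numbered name.
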(event OnComponentBeginOverlap(CollisionDetectPlayer)
  (params (OverlappedComponent :type Primitive%20Component%20Object%20Reference) (OtherActor :type Actor%20Object%20Reference) (OtherComp :type Primitive%20Component%20Object%20Reference) (OtherBodyIndex :type Integer) (bFromSweep :type Boolean) (SweepResult :type Hit%20Result%20Structure%20%28by%20ref%29))
  (bind _as_bp_player (CallFunction|GetPlayerReference))
  (bind _level (CallFunction|GetCurrentLevel))
  (bind _returnvalue (+ _level 1))
  (if (and (== OtherActor _as_bp_player) (Variables|Default|GetisActive))
    (Utilities|FlowControl|DoOnce false
      (:Completed
        (Utilities|FlowControl|Sequence
          (:then_0
            (bind _returnvalue_2 (SaveGame|LoadGamefromSlot "save"))
            (bind _asbp_save_game (Utilities|Casting|CastToBP_SaveGame _returnvalue_2))
            (Default|SetLevel _asbp_save_game _returnvalue)
            (Default|SetFruits _asbp_save_game (Variables|/Game/PixelAdventure/Characters/Player/BP_Player.BP_Player_C|GettotalCollectedFruitsOnCurrentLevel (CallFunction|GetPlayerReference)))
            (bind _newtrack_0 (Timeline|Timeline Play)
              (:Update
                (Rendering|Material|SetScalarParameterValue "/Game/PixelAdventure/Assets/Materials/ParametersCollection/MPC_amount.MPC_amount" "amount" _newtrack_0 :!class /Script/Engine.KismetMaterialLibrary))
              (:Finished
                (Utilities|FlowControl|Delay 0.2)
                (Game|OpenLevel(byName) (Utilities|String|StringToName (Utilities|String|Append "Level_" (Utilities|String|ToString(Integer) _returnvalue)))))))
          (:then_1
            (Variables|/Game/PixelAdventure/Characters/Player/BP_Player.BP_Player_C|SetcanReceiveDamage _as_bp_player false))
          (:then_2
            (Audio|SpawnSound2D "/Game/PixelAdventure/Assets/Audio/Effects/victory.victory" 1.0 1.0 0.0 0 true)))))))

(event Custom|enableFlag
  (bind _paperflipbook (Variables|Default|GetPaperFlipbook))
  (Variables|Default|SetisActive true)
  (Sprite|SetFlipbook _paperflipbook "/Game/PixelAdventure/Assets/Interactables/Checkpoint/actived/FB_Checkpoint_Actived.FB_Checkpoint_Actived")
  (Utilities|FlowControl|Delay (Class|PaperFlipbookComponent|GetFlipbookLength _paperflipbook))
  (Sprite|SetFlipbook _paperflipbook "/Game/PixelAdventure/Assets/Interactables/Checkpoint/idle/FB_Checkpoint_Actived_Idle.FB_Checkpoint_Actived_Idle"))

(event EventBeginPlay)

(event Collision|EventActorBeginOverlap
  (params (OtherActor :type Actor%20Object%20Reference)))

(event EventTick
  (params (DeltaSeconds :type Float%20%28single-precision%29)))

(fn ConstructionScript)