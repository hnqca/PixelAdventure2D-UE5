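; Spline path actor that walks an assigned character along its spline from BeginPlay, ping-ponging between the ends when looping is enabled.
; A timeline scaled to the set duration picks a target point on the spline.
; The character steers toward it with movement input and yaws to face it, while a FlipFlop alternates play and reverse.
; Chain-sprite trail and direct actor-transform logic exist but are disconnected.
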(event Custom|start%20movement%20along%20spline
  (bind _charactertomove (Variables|Default|GetCharacterToMove))
  (bind _spline (Variables|Default|GetSpline))
  (Components|Timeline|SetPlayRate (Variables|Default|GetTimeline_SplineMovement) (/ 1.0 (Variables|Default|GetdurationSplineMovement%20%28in%20seconds%29)))
  (Utilities|FlowControl|FlipFlop
    (:A
      (bind _transition (Timeline|Timeline_SplineMovement Play)
        (:Update
          (Pawn|Input|AddMovementInput _charactertomove (Math|Vector|Normalize (- (Spline|GetLocationatDistanceAlongSpline _spline (* _transition (Spline|GetSplineLength _spline)) "World") (Transformation|GetActorLocation (Variables|Default|GetCharacterToMove)))) 1.0 false)
          (Transformation|SetActorRotation (Variables|Default|GetCharacterToMove) (Math|Rotator|MakeRotator 0.0 0.0 (.yaw (Math|Rotator|FindLookatRotation (Transformation|GetActorLocation _charactertomove) (Spline|GetLocationatDistanceAlongSpline _spline (* _transition (Spline|GetSplineLength _spline)) "World"))))))
        (:Finished
          (if (Variables|Default|GetisLoopMovement)
            (CallFunction|StartMovementAlongSpline)))))
    (:B
      (Timeline|Timeline_SplineMovement Reverse))))

(event EventBeginPlay
  (CallFunction|StartMovementAlongSpline))

(event Collision|EventActorBeginOverlap
  (params (OtherActor :type Actor%20Object%20Reference)))

(event EventTick
  (params (DeltaSeconds :type Float%20%28single-precision%29)))

(fn ConstructionScript)

(fn SetChainTrail
  (for _index (range 0 (Math|Float|Floor (/ (Spline|GetSplineLength (Variables|Default|GetSpline)) (Variables|Default|GetOffsetChain))))
    (bind _returnvalue (AddComponent|AddPaperSpriteComponent false (Math|Conversions|ToTransform(Vector) (- (Spline|GetLocationatDistanceAlongSpline (Variables|Default|GetSpline) (* _index (Variables|Default|GetOffsetChain)) "Local") "0.000000,1.000000,0.000000"))))
    (Rendering|Components|Sprite|SetSprite _returnvalue (Variables|Default|GetSpriteChain))
    (Collision|SetCollisionEnabled _returnvalue "NoCollision")))