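; BP_SaveGame is the save object for Pixel Adventure, holding level progress, total fruits collected and total player deaths.
; SetLevel compares the given level with the stored one and writes it only when that check fails, apparently keeping the highest level reached.
; SetFruits and SetPlayerTotalDeaths add increments to running totals.
; Each write immediately saves the object itself to the "save" slot.
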(fn SetLevel
  (params (level :type Integer))
  (if (>= (Variables|Default|Getlevel) level)
    _
    (else
      (Variables|Default|Setlevel level)
      (SaveGame|SaveGametoSlot self "save")))
  (return (>= (Variables|Default|Getlevel) level)))

(fn SetFruits
  (params (total%20fruits%20to%20increment :type Integer))
  (bind _output_get (Variables|Default|SettotalFruitsCollected (+ total%20fruits%20to%20increment (Variables|Default|GettotalFruitsCollected))))
  (SaveGame|SaveGametoSlot self "save")
  (return _output_get))

(fn SetPlayerTotalDeaths
  (params (quantity%20to%20increment :type Integer))
  (bind _output_get (Variables|Default|SetplayerTotalDeaths (+ quantity%20to%20increment (Variables|Default|GetplayerTotalDeaths))))
  (SaveGame|SaveGametoSlot self "save")
  (return _output_get))