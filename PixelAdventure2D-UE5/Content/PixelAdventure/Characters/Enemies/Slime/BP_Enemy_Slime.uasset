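; Slime enemy Blueprint that periodically drops poison traps while it is alive.
; On BeginPlay it starts a looping timer whose interval is randomized once, so each slime keeps its own steady drop rate.
; Each timer tick spawns a poison trap actor at a scene component's transform, ignoring collisions, unless the slime is dead.
; Other behavior is left to the parent class.
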(event Custom|spawnPoison
  (if (not (Variables|Default|GetisDead))
    (Game|SpawnActorfromClass "/Game/PixelAdventure/Actors/Traps/BP_Trap_Slime_Poison.BP_Trap_Slime_Poison_C" (Transformation|GetWorldTransform (Variables|Default|GetsceneLocationSpawnPoison)) "AlwaysSpawn" "MultiplyWithRoot" 0 0)))

(event EventBeginPlay
  (|CallParentFunction)
  (Utilities|Time|SetTimerbyEvent (delegate Custom|spawnPoison) (Math|Random|RandomFloatinRange 0.5 1.2) true))

(event Collision|EventActorBeginOverlap
  (params (OtherActor :type Actor%20Object%20Reference))
  (|CallParentFunction OtherActor) ; This node is disabled and will not be called.\nDrag off pins to build functionality.
)

(event EventTick
  (params (DeltaSeconds :type Float%20%28single-precision%29))
  (|CallParentFunction DeltaSeconds) ; This node is disabled and will not be called.\nDrag off pins to build functionality.
)

(fn ConstructionScript
  (|CallParentFunction))