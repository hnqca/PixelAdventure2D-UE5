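; Radish enemy that starts out hovering, drops to the ground when first damaged, and dies when damaged again.
; A timeline lerps its Z around the spawn position while flying.
; The first hit stops the timeline, switches movement to Walking, bounces the player with sound and camera shake, and enables walking patrol shortly after landing.
; A DoOnce, reset after a short delay, blocks repeated hits until a later one calls OnDeath.
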(event Custom|startFlyMovement
  (bind _originalactorlocation (Variables|Default|GetoriginalActorLocation))
  (bind _transition (Timeline|Timeline_0 PlayFromStart)
    (:Update
      (Transformation|SetActorLocation (Math|Vector|MakeVector (.x _originalactorlocation) (.y _originalactorlocation) (Math|Float|Lerp (.z _originalactorlocation) (+ (.z (Variables|Default|GetoriginalActorLocation)) (Variables|Default|GetNew%20Location%20Z)) _transition)) true true))))

(event EventBeginPlay
  (|CallParentFunction)
  (Variables|Default|SetoriginalActorLocation (Transformation|GetActorLocation))
  (CallFunction|StartFlyMovement))

(event Collision|EventActorBeginOverlap
  (params (OtherActor :type Actor%20Object%20Reference))
  (|CallParentFunction OtherActor) ; This node is disabled and will not be called.\nDrag off pins to build functionality.
)

(event EventTick
  (params (DeltaSeconds :type Float%20%28single-precision%29))
  (|CallParentFunction DeltaSeconds) ; This node is disabled and will not be called.\nDrag off pins to build functionality.
)

(event Game|Damage|EventAnyDamage
  (params (Damage :type Float%20%28single-precision%29) (DamageType :type Damage%20Type%20Object%20Reference) (InstigatedBy :type Controller%20Object%20Reference) (DamageCauser :type Actor%20Object%20Reference))
  (bind _as_bp_player (CallFunction|GetPlayerReference))
  (bind _originalactorlocation (Variables|Default|GetoriginalActorLocation))
  (Utilities|FlowControl|DoOnce false :!label _label
    (:Completed
      (Class|PaperZDAnimInstance|JumptoNode (Variables|/Script/PaperZD.PaperZDAnimationComponent|GetAnimInstance (Variables|Default|GetAnimationComponent)) "onReceiveDamage" "None")
      (if (Variables|Default|GetisFlying)
        (Utilities|FlowControl|Sequence
          (:then_0
            (bind _transition (Timeline|Timeline_0 Stop)
              (:Update
                (Transformation|SetActorLocation (Math|Vector|MakeVector (.x _originalactorlocation) (.y _originalactorlocation) (Math|Float|Lerp (.z _originalactorlocation) (+ (.z (Variables|Default|GetoriginalActorLocation)) (Variables|Default|GetNew%20Location%20Z)) _transition)) true true))))
          (:then_1
            (Variables|Default|SetisFlying false)
            (Variables|/Script/Engine.CharacterMovementComponent|SetDefaultLandMovementMode (Variables|Character|GetCharacterMovement) "MOVE_Walking")
            (Pawn|Components|CharacterMovement|SetMovementMode (Variables|Character|GetCharacterMovement) "MOVE_Walking" 0)
            (Utilities|FlowControl|Delay 0.3)
            (goto _label Reset))
          (:then_2
            (Character|LaunchCharacter _as_bp_player (Math|Vector|MakeVector 0.0 0.0 (* (Variables|/Script/Engine.CharacterMovementComponent|GetJumpZVelocity (Variables|/Script/Engine.Character|GetCharacterMovement _as_bp_player)) 1.05)) true true)
            (Audio|PlaySound2D "/Game/PixelAdventure/Assets/Audio/Effects/enemyDamage.enemyDamage" 1.0 1.0 0.0 0 0)
            (bind _returnvalue (Actor|GetActorOfClass "/Game/PixelAdventure/Actors/BP_CameraLevel.BP_CameraLevel_C"))
            (Camera|PlayWorldCameraShake "/Game/PixelAdventure/Core/CameraShake/CS_ApplyDamageEnemy.CS_ApplyDamageEnemy_C" (Transformation|GetWorldLocation (Variables|/Script/Engine.Actor|GetRootComponent _returnvalue)) 55.0 1e+01)))
        (else
          (CallFunction|OnDeath DamageCauser))))))

(event EventOnLanded
  (params (Hit :type Hit%20Result%20Structure%20%28by%20ref%29))
  (Utilities|FlowControl|Delay 0.2)
  (Variables|Default|SetcanPatrolWalking true))

(fn ConstructionScript
  (|CallParentFunction))