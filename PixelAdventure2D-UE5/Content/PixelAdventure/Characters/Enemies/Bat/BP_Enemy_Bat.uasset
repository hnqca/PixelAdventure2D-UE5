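; Bat enemy that sleeps until the player first enters its detection collision, then chases them.
; Detection wakes it, switches movement to Falling and, after a short delay, opens a Tick-driven Gate.
; While the Gate is open, it moves straight toward the player and yaws to face them.
; The first damage received closes the Gate, restores gravity, plays the hit animation and calls OnDeath with the damage causer.
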(event OnComponentBeginOverlap(collisionDetectPlayer)
  (params (OverlappedComponent :type Primitive%20Component%20Object%20Reference) (OtherActor :type Actor%20Object%20Reference) (OtherComp :type Primitive%20Component%20Object%20Reference) (OtherBodyIndex :type Integer) (bFromSweep :type Boolean) (SweepResult :type Hit%20Result%20Structure%20%28by%20ref%29))
  (if (== OtherActor (CallFunction|GetPlayerReference))
    (Utilities|FlowControl|DoOnce false
      (:Completed
        (Variables|Default|SetisSleeping false)
        (Utilities|FlowControl|Sequence
          (:then_0
            (Utilities|FlowControl|Delay 0.8)
            (CallFunction|StartFollowPlayer))
          (:then_1
            (Pawn|Components|CharacterMovement|SetMovementMode (Variables|Character|GetCharacterMovement) "MOVE_Falling" 0)))))))

(event Custom|startFollowPlayer
  (Variables|Default|SetisSleeping false)
  (Variables|Default|SetisFollowingPlayer false)
  (Utilities|FlowControl|Gate true) ; enters at Open
)

(event Custom|stopFollowPlayer
  (Variables|Default|SetisFollowingPlayer false)
  (Utilities|FlowControl|Gate true) ; enters at Close
)

(event EventBeginPlay
  (|CallParentFunction) ; This node is disabled and will not be called.\nDrag off pins to build functionality.
)

(event Collision|EventActorBeginOverlap
  (params (OtherActor :type Actor%20Object%20Reference))
  (|CallParentFunction OtherActor) ; This node is disabled and will not be called.\nDrag off pins to build functionality.
)

(event EventTick
  (params (DeltaSeconds :type Float%20%28single-precision%29))
  (|CallParentFunction DeltaSeconds)
  (Utilities|FlowControl|Gate true
    (:Exit
      ;[1 1 1] Move o inimigo até a direção do jogador no mundo
      (Pawn|Input|AddMovementInput (Math|Vector|Normalize (- (Transformation|GetActorLocation (CallFunction|GetPlayerReference)) (Transformation|GetActorLocation self))) 1.0 false)
      ;[1 1 1] rotaciona o inimigo para a direção do jogador
      (Transformation|SetActorRotation (Math|Rotator|MakeRotator 0.0 0.0 (.yaw (Math|Rotator|FindLookatRotation (Transformation|GetActorLocation) (Transformation|GetActorLocation (CallFunction|GetPlayerReference)))))))))

(event Game|Damage|EventAnyDamage
  (params (Damage :type Float%20%28single-precision%29) (DamageType :type Damage%20Type%20Object%20Reference) (InstigatedBy :type Controller%20Object%20Reference) (DamageCauser :type Actor%20Object%20Reference))
  (Utilities|FlowControl|DoOnce false
    (:Completed
      (CallFunction|StopFollowPlayer)
      (Variables|/Script/Engine.CharacterMovementComponent|SetGravityScale (Variables|Character|GetCharacterMovement) 1.0)
      (CallFunction|StartAnimReceiveDamage)
      (CallFunction|OnDeath DamageCauser))))

(fn ConstructionScript
  (|CallParentFunction))