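; Fat Bird enemy that hovers vertically around its spawn point and drops when the player enters its detection collision.
; A timeline drives the hover; detection stops it and switches movement from Flying to Walking so the bird falls.
; After landing it pauses, lerps back to its origin in Flying mode, then resumes hovering and re-arms detection.
; Damage stops both timelines, restores Walking, and triggers the hit animation and death.
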(event OnComponentBeginOverlap(collisionDetectPlayerToFall)
  (params (OverlappedComponent :type Primitive%20Component%20Object%20Reference) (OtherActor :type Actor%20Object%20Reference) (OtherComp :type Primitive%20Component%20Object%20Reference) (OtherBodyIndex :type Integer) (bFromSweep :type Boolean) (SweepResult :type Hit%20Result%20Structure%20%28by%20ref%29))
  (if (== OtherActor (CallFunction|GetPlayerReference))
    (Utilities|FlowControl|DoOnce false
      (:Completed
        (Variables|/Script/Engine.CharacterMovementComponent|SetDefaultLandMovementMode (Variables|Character|GetCharacterMovement) "MOVE_Walking")
        (Pawn|Components|CharacterMovement|SetMovementMode (Variables|Character|GetCharacterMovement) "MOVE_Walking" 0)
        (Audio|Components|Audio|Stop (Variables|Default|GetTimeline_FlyMovement))))))

(event Custom|startFlyMovement
  (bind _originalactorworldlocation (Variables|Default|GetoriginalActorWorldLocation))
  (bind _transition (Timeline|Timeline_FlyMovement PlayFromStart)
    (:Update
      (Transformation|SetActorLocation (Math|Vector|MakeVector (.x _originalactorworldlocation) (.y _originalactorworldlocation) (Math|Float|Lerp (.z _originalactorworldlocation) (+ (.z (Variables|Default|GetoriginalActorWorldLocation)) (Variables|Default|GetoffsetActorLocationZ)) _transition)) true true))))

(event Custom|resetDoOnceDetectPlayerCollision
  (Utilities|FlowControl|DoOnce false) ; enters at Reset
)

(event EventBeginPlay
  (|CallParentFunction)
  (Variables|Default|SetoriginalActorWorldLocation (Transformation|GetActorLocation))
  (CallFunction|StartFlyMovement))

(event Collision|EventActorBeginOverlap
  (params (OtherActor :type Actor%20Object%20Reference))
  (|CallParentFunction OtherActor) ; This node is disabled and will not be called.\nDrag off pins to build functionality.
)

(event EventTick
  (params (DeltaSeconds :type Float%20%28single-precision%29)))

(event EventOnLanded
  (params (Hit :type Hit%20Result%20Structure%20%28by%20ref%29))
  (Utilities|FlowControl|Delay 1.0)
  (Variables|/Script/Engine.CharacterMovementComponent|SetDefaultLandMovementMode (Variables|Character|GetCharacterMovement) "MOVE_Flying")
  (Pawn|Components|CharacterMovement|SetMovementMode (Variables|Character|GetCharacterMovement) "MOVE_Flying" 0)
  (Components|Timeline|SetPlayRate (Variables|Default|GetTimeline_0) (/ 1.0 1.0))
  (bind _transition (Timeline|Timeline_0 PlayFromStart)
    (:Update
      (Transformation|SetActorLocation (Math|Vector|Lerp(Vector) (Transformation|GetActorLocation) (Variables|Default|GetoriginalActorWorldLocation) (/ _transition 8.0)) false false))
    (:Finished
      (Development|PrintString "Hello")
      (Components|Timeline|PlayfromStart (Variables|Default|GetTimeline_FlyMovement))
      (CallFunction|ResetDoOnceDetectPlayerCollision))))

(event Game|Damage|EventAnyDamage
  (params (Damage :type Float%20%28single-precision%29) (DamageType :type Damage%20Type%20Object%20Reference) (InstigatedBy :type Controller%20Object%20Reference) (DamageCauser :type Actor%20Object%20Reference))
  (Utilities|FlowControl|DoOnce false
    (:Completed
      (Utilities|FlowControl|Sequence
        (:then_0
          (Audio|Components|Audio|Stop (Variables|Default|GetTimeline_FlyMovement))
          (Audio|Components|Audio|Stop (Variables|Default|GetTimeline_0))
          (Variables|/Script/Engine.CharacterMovementComponent|SetDefaultLandMovementMode (Variables|Character|GetCharacterMovement) "MOVE_Walking")
          (Pawn|Components|CharacterMovement|SetMovementMode (Variables|Character|GetCharacterMovement) "MOVE_Walking" 0))
        (:then_1
          (CallFunction|StartAnimReceiveDamage)
          (CallFunction|OnDeath DamageCauser))))))

(fn ConstructionScript
  (|CallParentFunction))