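; Rino enemy Blueprint for Pixel Adventure that charges horizontally and recoils off walls.
; Tick feeds movement input along X through a Gate, with direction set by IsMovingRight.
; A hit with a purely horizontal normal launches it back and up, toggles direction via FlipFlop, and closes the Gate.
; After a short Delay it rotates to face the new direction and reopens the Gate; every hit also prints its normal X.
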(event EventBeginPlay
  (|CallParentFunction))

(event Collision|EventActorBeginOverlap
  (params (OtherActor :type Actor%20Object%20Reference))
  (|CallParentFunction OtherActor))

(event EventTick
  (params (DeltaSeconds :type Float%20%28single-precision%29))
  (Utilities|FlowControl|Gate false
    (:Exit
      (Pawn|Input|AddMovementInput (Math|Vector|MakeVector (select (Variables|Default|GetisMovingRight?) 1.0 -1.0) 0.0 0.0) 1.0 false))))

(event Collision|EventHit
  (params (MyComp :type Primitive%20Component%20Object%20Reference) (Other :type Actor%20Object%20Reference) (OtherComp :type Primitive%20Component%20Object%20Reference) (bSelfMoved :type Boolean) (HitLocation :type Vector :default "0, 0, 0") (HitNormal :type Vector :default "0, 0, 0") (NormalImpulse :type Vector :default "0, 0, 0") (Hit :type Hit%20Result%20Structure%20%28by%20ref%29))
  (bind _x (Class|KismetMathLibrary|BreakVector3f HitNormal))
  (bind _returnvalue (== _x 1.0))
  (Development|PrintString (Utilities|String|ToString(Float) _x))
  (if (or _returnvalue (== _x -1.0))
    (Utilities|FlowControl|Sequence
      (:then_0
        (Character|LaunchCharacter (Math|Vector|MakeVector (select _returnvalue 1e+02 -1e+02) 0.0 2.5e+02) true true)
        (bind _isa (Utilities|FlowControl|FlipFlop)
          (:A
            _)
          (:B
            _))
        (bind _output_get (Variables|Default|SetisMovingRight? _isa))
        (Utilities|FlowControl|Delay 1.5)
        (CallFunction|ChangeActorRotationbyMovingDirection _output_get)
        (Utilities|FlowControl|Gate false) ; enters at Open
      )
      (:then_1
        (Utilities|FlowControl|Gate false) ; enters at Close
      ))))

(fn ConstructionScript)