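; Side-scrolling enemy character for Pixel Adventure that patrols along the X axis, damages the player on overlap and dies from a single hit.
; Tick drives walking, with a FlipFlop reversing direction on capsule hits or failed ledge checks, the latter after an optional idle pause.
; Death plays the hurt animation and sound, disables collision, launches and rotates the body by timeline before destruction, and bounces a player attacker with camera shake.
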(event OnComponentBeginOverlap(collisionApplyDamage)
  (params (OverlappedComponent :type Primitive%20Component%20Object%20Reference) (OtherActor :type Actor%20Object%20Reference) (OtherComp :type Primitive%20Component%20Object%20Reference) (OtherBodyIndex :type Integer) (bFromSweep :type Boolean) (SweepResult :type Hit%20Result%20Structure%20%28by%20ref%29))
  (bind _as_bp_player (CallFunction|GetPlayerReference))
  ;[1 1 1 1 22] Aplica dano ao jogador
  (if (Math|Boolean|ANDBoolean (== OtherActor _as_bp_player) (Variables|Default|GetcanApplyDamage) (not (Variables|Default|GetisDead)) (Variables|/Game/PixelAdventure/Characters/Player/BP_Player.BP_Player_C|GetcanReceiveDamage _as_bp_player))
    (Game|Damage|ApplyDamage _as_bp_player 1.0 0 0)))

(event Custom|setWalkingPatrol
  ;[1 1 1] Walking Patroll
  ;;[1 1 1] Apenas se o inimigo estiver vivo
  (Utilities|FlowControl|Sequence
    (:then_0
      ;;[0.8275 0 1] Direção do movemento atual
      (Pawn|Input|AddMovementInput "1.000000,0.000000,0.000000" (select (Variables|Default|GetisMovingRight?) 1.0 -1.0) false))
    (:then_1
      ;;[0 1 0.2275] Alterna o movement se bater em algo
      (Collision|AssignOnComponentHit (Variables|Default|GetCapsuleComponent) (delegate Custom|onHitComponent)))
    (:then_2
      (bind _cancontinuewalking_ (CallFunction|CheckLedgePatrolWalking))
      (if (not _cancontinuewalking_)
        (if (== (Variables|Default|GetpatrolWalkingIdleDelay) 0.0)
          _
          (else
            (Variables|Default|SetcanPatrolWalking false)
            (Utilities|FlowControl|Delay (Variables|Default|GetpatrolWalkingIdleDelay))
            (Variables|Default|SetcanPatrolWalking true)))
        (bind _isa (Utilities|FlowControl|FlipFlop)
          (:A
            _)
          (:B
            _))
        (CallFunction|ChangeActorRotationbyMovingDirection _isa)))))

(event Custom|onDeath
  (params (Damage%20Causer :type Actor%20Object%20Reference))
  (bind _as_bp_player (CallFunction|GetPlayerReference))
  (Utilities|FlowControl|DoOnce false
    (:Completed
      (Utilities|FlowControl|Sequence
        (:then_0
          (Variables|Default|SetcanPatrolWalking false)
          (Variables|Default|SetisDead true)
          (Collision|SetActorEnableCollision false)
          (Utilities|FlowControl|Sequence
            (:then_0
              (Character|LaunchCharacter (Math|Vector|MakeVector 0.0 5e+01 2.5e+02) true true)
              (bind _newtrack_0 (Timeline|Timeline Play)
                (:Update
                  (Transformation|SetActorRotation (Math|Rotator|MakeRotator 0.0 _newtrack_0 0.0)))
                (:Finished
                  (Actor|DestroyActor))))
            (:then_1
              (if (== Damage%20Causer (CallFunction|GetPlayerReference))
                (Default|Launch _as_bp_player 1.05)
                (Default|StartCameraShakeApplyDamage _as_bp_player)
                (Audio|PlaySound2D "/Game/PixelAdventure/Assets/Audio/Effects/enemyDamage.enemyDamage" 1.0 1.0 0.0 0 0)))))
        (:then_1
          (Components|DestroyComponent (Variables|Default|GetcollisionApplyDamage)))))))

(event Custom|onHitComponent
  (params (HitComponent :type Primitive%20Component%20Object%20Reference) (OtherActor :type Actor%20Object%20Reference) (OtherComp :type Primitive%20Component%20Object%20Reference) (NormalImpulse :type Vector) (Hit :type Hit%20Result%20Structure%20%28by%20ref%29))
  ;[1 1 1] Walking Patroll
  ;;[0 1 0.2275] Alterna o movement se bater em algo
  (bind _isa (Utilities|FlowControl|FlipFlop)
    (:A
      _)
    (:B
      _))
  (CallFunction|ChangeActorRotationbyMovingDirection _isa))

(event Custom|startAnimReceiveDamage
  (Class|PaperZDAnimInstance|JumptoNode (Variables|/Script/PaperZD.PaperZDAnimationComponent|GetAnimInstance (Variables|Default|GetAnimationComponent)) "onReceiveDamage" "None")
  (Audio|PlaySound2D "/Game/PixelAdventure/Assets/Audio/Effects/enemyDamage.enemyDamage" 1.0 1.0 0.0 0 0))

(event Custom|changeActorRotationByMovingDirection
  (params (isMovingRight? :type Boolean))
  ;[1 1 1] Walking Patroll
  (bind _output_get (Variables|Default|SetisMovingRight? isMovingRight?))
  (Transformation|SetActorRotation (Math|Rotator|MakeRotator 0.0 0.0 (select _output_get 0.0 1.8e+02))))

(event EventBeginPlay
  (Variables|Default|SetisMovingRight? (== (.yaw (Transformation|GetActorRotation)) 0.0)))

(event Collision|EventActorBeginOverlap
  (params (OtherActor :type Actor%20Object%20Reference)))

(event EventTick
  (params (DeltaSeconds :type Float%20%28single-precision%29))
  (bind _returnvalue (CallFunction|CheckCanPatrolWalking))
  (if _returnvalue
    (CallFunction|SetWalkingPatrol)))

(event Game|Damage|EventAnyDamage
  (params (Damage :type Float%20%28single-precision%29) (DamageType :type Damage%20Type%20Object%20Reference) (InstigatedBy :type Controller%20Object%20Reference) (DamageCauser :type Actor%20Object%20Reference))
  (Utilities|FlowControl|DoOnce false
    (:Completed
      (CallFunction|StartAnimReceiveDamage)
      (CallFunction|OnDeath DamageCauser))))

(fn ConstructionScript)

(fn CheckLedgePatrolWalking
  (return (and (.bWalkableFloor (Utilities|Struct|BreakFindFloorResult (Variables|/Script/Engine.CharacterMovementComponent|GetCurrentFloor (Variables|Character|GetCharacterMovement)))) (> (Utilities|Array|Length (Collision|GetOverlappingActors (Variables|Default|GetcollisionPatrolWalkingCheck) 0 :!class /Script/Engine.PrimitiveComponent)) 0))))

(fn ChangeSpriteDirection
  (bind _sprite (Variables|Default|GetSprite))
  (bind _returnvalue (Transformation|GetWorldScale _sprite))
  (Transformation|SetWorldScale3D _sprite (Math|Vector|MakeVector (* (.x _returnvalue) -1.0) (.y _returnvalue) (.z _returnvalue))))

(fn CheckCanPatrolWalking
  (return (and (Variables|Default|GetcanPatrolWalking) (not (AI|Components|NavMovement|IsFalling (Variables|Character|GetCharacterMovement))))))