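; Plant enemy Blueprint that triggers its attack animation when the player enters its detection collision.
; The overlap event ignores other actors and does nothing once the plant is dead.
; A valid overlap jumps the animation instance to its attack node, with a DoOnce reset after a short delay acting as a cooldown.
; The graph itself contains no projectile or damage logic.
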(event OnComponentBeginOverlap(collisionDetectPlayerToAttack)
  (params (OverlappedComponent :type Primitive%20Component%20Object%20Reference) (OtherActor :type Actor%20Object%20Reference) (OtherComp :type Primitive%20Component%20Object%20Reference) (OtherBodyIndex :type Integer) (bFromSweep :type Boolean) (SweepResult :type Hit%20Result%20Structure%20%28by%20ref%29))
  (if (and (== OtherActor (CallFunction|GetPlayerReference)) (not (Variables|Default|GetisDead)))
    (Utilities|FlowControl|DoOnce false :!label _label
      (:Completed
        (Utilities|FlowControl|Sequence
          (:then_0
            (Utilities|FlowControl|Delay 0.4)
            (goto _label Reset))
          (:then_1
            (Class|PaperZDAnimInstance|JumptoNode (Variables|/Script/PaperZD.PaperZDAnimationComponent|GetAnimInstance (Variables|Default|GetAnimationComponent)) "onAttack" "None")))))))

(event EventBeginPlay
  (|CallParentFunction) ; This node is disabled and will not be called.\nDrag off pins to build functionality.
)

(event Collision|EventActorBeginOverlap
  (params (OtherActor :type Actor%20Object%20Reference))
  (|CallParentFunction OtherActor) ; This node is disabled and will not be called.\nDrag off pins to build functionality.
)

(event EventTick
  (params (DeltaSeconds :type Float%20%28single-precision%29))
  (|CallParentFunction DeltaSeconds) ; This node is disabled and will not be called.\nDrag off pins to build functionality.
)

(fn ConstructionScript
  (|CallParentFunction))