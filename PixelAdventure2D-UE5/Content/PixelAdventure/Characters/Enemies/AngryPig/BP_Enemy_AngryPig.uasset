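; Angry pig enemy Blueprint that takes two hits to kill, changing state after the first.
; The first hit plays the damage animation, launches the player with a camera shake, sets the pig angry and switches its walk speed to the angry value.
; A DoOnce gates damage handling and resets after that hit, so the next hit calls OnDeath with the damage causer.
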(event EventBeginPlay
  (|CallParentFunction) ; This node is disabled and will not be called.\nDrag off pins to build functionality.
)

(event Collision|EventActorBeginOverlap
  (params (OtherActor :type Actor%20Object%20Reference))
  (|CallParentFunction OtherActor) ; This node is disabled and will not be called.\nDrag off pins to build functionality.
)

(event EventTick
  (params (DeltaSeconds :type Float%20%28single-precision%29))
  (|CallParentFunction DeltaSeconds) ; This node is disabled and will not be called.\nDrag off pins to build functionality.
)

(event Game|Damage|EventAnyDamage
  (params (Damage :type Float%20%28single-precision%29) (DamageType :type Damage%20Type%20Object%20Reference) (InstigatedBy :type Controller%20Object%20Reference) (DamageCauser :type Actor%20Object%20Reference))
  (bind _as_bp_player (CallFunction|GetPlayerReference))
  (Utilities|FlowControl|DoOnce false :!label _label
    (:Completed
      (CallFunction|StartAnimReceiveDamage)
      (if (Variables|Default|GetbAngry)
        (CallFunction|OnDeath DamageCauser)
        (else
          (Utilities|FlowControl|Sequence
            (:then_0
              (Default|Launch _as_bp_player 1.05)
              (Default|StartCameraShakeApplyDamage _as_bp_player))
            (:then_1
              (Variables|Default|SetbAngry true)
              (Variables|/Script/Engine.CharacterMovementComponent|SetMaxWalkSpeed (Variables|Character|GetCharacterMovement) (Variables|Default|GetangryVelocityWalk))
              (goto _label Reset))))))))

(fn ConstructionScript
  (|CallParentFunction))