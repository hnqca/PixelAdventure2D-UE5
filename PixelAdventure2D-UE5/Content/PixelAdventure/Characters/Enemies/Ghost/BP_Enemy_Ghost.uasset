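; Ghost enemy Blueprint that periodically switches between visible and invisible states and dies on the first damage it receives.
; A looping timer started on BeginPlay drives a FlipFlop that sets IsInvisible, with CanApplyDamage as its inverse.
; AnyDamage passes through a DoOnce, jumps the animation instance to its damage-reaction node and calls OnDeath with the damage causer.
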(event Custom|toggleStatusVisibility
  (bind _isa (Utilities|FlowControl|FlipFlop)
    (:A
      _)
    (:B
      _))
  (bind _output_get (Variables|Default|SetisInvisible _isa))
  (Variables|Default|SetcanApplyDamage (not _output_get)))

(event EventBeginPlay
  (|CallParentFunction)
  (Utilities|Time|SetTimerbyEvent (delegate Custom|toggleStatusVisibility) (Variables|Default|GetsecondsToggleVisibility) true))

(event Collision|EventActorBeginOverlap
  (params (OtherActor :type Actor%20Object%20Reference))
  (|CallParentFunction OtherActor) ; This node is disabled and will not be called.\nDrag off pins to build functionality.
)

(event EventTick
  (params (DeltaSeconds :type Float%20%28single-precision%29))
  (|CallParentFunction DeltaSeconds) ; This node is disabled and will not be called.\nDrag off pins to build functionality.
)

(event Game|Damage|EventAnyDamage
  (params (Damage :type Float%20%28single-precision%29) (DamageType :type Damage%20Type%20Object%20Reference) (InstigatedBy :type Controller%20Object%20Reference) (DamageCauser :type Actor%20Object%20Reference))
  (Utilities|FlowControl|DoOnce false
    (:Completed
      (Class|PaperZDAnimInstance|JumptoNode (Variables|/Script/PaperZD.PaperZDAnimationComponent|GetAnimInstance (Variables|Default|GetAnimationComponent)) "onReceiveDamage" "None")
      (CallFunction|OnDeath DamageCauser))))

(fn ConstructionScript
  (|CallParentFunction))